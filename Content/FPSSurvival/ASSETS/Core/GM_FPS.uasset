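; GM_FPS is the game mode for a wave-based FPS zombie survival game, starting the first wave on BeginPlay.
; Each wave spawns a zombie count scaled by the wave number, split between two spawn locations.
; ZombieKilled decrements the remaining count; when a wave clears, it advances after showing wave UI on BP_Character and a short delay.
; Clearing the final wave shows the win UI on the player character.
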(event `self.ReceiveBeginPlay`
  (`self.StartGame`))

(event `WaveStart`
  ;[0.04057 0.06476 0.15 0.5] Start Next Wave
  (bind _asbp_character (cast `/Game/FPSSurvival/ASSETS/Core/BP_Character` (`GameplayStatics.GetPlayerCharacter` 0)))
  (`/Game/FPSSurvival/ASSETS/Core/BP_Character.ShowWaveUI` _asbp_character (`self.CurrentWave`))
  (`KismetSystemLibrary.Delay` 5.0)
  (`self.SpawnZombies`))

(event `StartGame`
  (`self.SpawnZombies`))

(event `SpawnZombies`
  ;[0.1498 0.01841 0.15 0.5] Spawn Zombies
  (bind _output_get (set `self.ZombieTotal` (* (`self.CurrentWave`) 8)))
  (set `self.ZombiesLeft` _output_get)
  (for _index (range (+ _output_get 1))
    (if (== _index (/ (`self.ZombieTotal`) 2))
      (break)
      (else
        (`|SpawnActorFromClass` "/Game/FPSSurvival/ASSETS/Core/BP_Zombie.BP_Zombie_C" (`self.SpawnLocation1`) "Undefined" "MultiplyWithRoot" null null))))
  (for _ (range 1 (+ (/ (`self.ZombieTotal`) 2) 1))
    (`|SpawnActorFromClass` "/Game/FPSSurvival/ASSETS/Core/BP_Zombie.BP_Zombie_C" (`self.SpawnLocation2`) "Undefined" "MultiplyWithRoot" null null)))

(event `ZombieKilled`
  ;[0.15 0 0 0.5] Zombie Killed
  (bind _result (`/Engine/EditorBlueprintResources/StandardMacros.DecrementInt` (`self.ZombiesLeft`))
    (:`  `
      (if (== _result 0)
        (`self.WaveIncrement`)))))

(event `WaveIncrement`
  ;[0.09915 0.3882 0.4219 0.5] Update Wave
  (if (== (`self.CurrentWave`) (`self.MaxWaves`))
    (`self.PlayerWins`)
    (else
      (`/Engine/EditorBlueprintResources/StandardMacros.IncrementInt` (`self.CurrentWave`)
        (:`  `
          (`self.WaveStart`))))))

(event `PlayerWins`
  ;[0.07356 0.15 0.09795 0.5] Win Logic
  (bind _asbp_character (cast `/Game/FPSSurvival/ASSETS/Core/BP_Character` (`GameplayStatics.GetPlayerCharacter` 0)))
  (`/Game/FPSSurvival/ASSETS/Core/BP_Character.ShowWinUI` _asbp_character))

(fn `UserConstructionScript`)