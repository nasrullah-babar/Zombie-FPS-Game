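; BP_Zombie is a survival FPS enemy that moves toward player controller 0, looping between chase and melee, with walk speed set on sight.
; A punch montage notify triggers a sphere overlap at Arrow1 that damages BP_Character, with a debug sphere drawn.
; Point damage lowers Health, but the post-hit check calls Death when Health is still zero or above.
; Death stumbles, loosens collision, notifies GM_FPS of the kill and destroys the actor after a delay.
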(event `self.PawnSensing.OnSeePawn`
  (params (Pawn :type "Pawn Object Reference"))
  (set `CharacterMovementComponent.MaxWalkSpeed` 360.0 (`self.CharacterMovement`)))

(event `self.ReceiveBeginPlay`
  (`self.RunToPlayer`))

(event `RunToPlayer`
  (if (not (`self.isDead`))
    (`|AIMoveTo` self (0.0 0.0 0.0) (`GameplayStatics.GetPlayerController` 0) 40.0
      (:`OnSuccess`
        (`self.AttackPlayer`))
      (:`OnFail`
        (`self.RunToPlayer`)))))

(event `AttackPlayer`
  (bind _returnvalue (`SceneComponent.K2_GetComponentLocation` (`self.Arrow1`)))
  ;[0.1495 0.15 0.02403 0.5] Attack Player logic which allows the zombies to attack us
  (`|PlayMontage` (`self.Mesh`) "/Game/Fab/Zombie_Number_4_-_Animated/Animations/Punch_Montage.Punch_Montage"
    (:`OnCompleted`
      (`self.RunToPlayer`))
    (:`OnNotifyBegin`
      (`GameplayStatics.PlaySoundAtLocation` "/Game/FPSSurvival/ASSETS/Sounds/SC_Attack.SC_Attack" (`self.K2_GetActorLocation`) (struct) 1.0 1.0 0.0 null null null null)
      (bind (_outactors _returnvalue_2) (`KismetSystemLibrary.SphereOverlapActors` _returnvalue 80.0 (`|MakeArray` "ObjectTypeQuery3" :!type "EObjectTypeQuery Enum") "/Game/FPSSurvival/ASSETS/Core/BP_Character.BP_Character_C" (`|MakeArray` self :!type "Actor Object Reference")))
      (`KismetSystemLibrary.DrawDebugSphere` _returnvalue 80.0 12 (struct :`R` 0.463542 :`G` 0.003205 :`B` 0.040136 :`A` 1.0) 10.0)
      (if _returnvalue_2
        (for _array_element _outactors
          (`GameplayStatics.ApplyDamage` _array_element 20.0 (`self.GetController`) self "/Script/Engine.DamageType"))))))

(event `self.ReceivePointDamage`
  (params (Damage :type "Float (single-precision)") (DamageType :type "DamageType Object Reference") (HitLocation :type "Vector Structure") (HitNormal :type "Vector Structure") (HitComponent :type "PrimitiveComponent Object Reference") (BoneName :type Name) (ShotFromDirection :type "Vector Structure") (InstigatedBy :type "Controller Object Reference") (DamageCauser :type "Actor Object Reference") (HitInfo :type "HitResult Structure (by ref)"))
  (if (`self.isDead`)
    _
    (elif (<= (`self.Health`) 0.0)
      (`self.Death`)
      (else
        (bind _output_get (set `self.Health` (- (`self.Health`) Damage)))
        (`KismetSystemLibrary.PrintString` (`KismetStringLibrary.Conv_DoubleToString` _output_get))
        (if (<= 0.0 _output_get)
          (`self.Death`)
          (else
            (`|PlayMontage` (`self.Mesh`) "/Game/Fab/Zombie_Number_4_-_Animated/Animations/Take_Hit_Montage.Take_Hit_Montage")))))))

(event `Death`
  (set `self.isDead` true)
  (`MovementComponent.StopMovementImmediately` (`self.CharacterMovement`))
  (`|PlayMontage` (`self.Mesh`) "/Game/Fab/Zombie_Number_4_-_Animated/Animations/Stumble_Montage.Stumble_Montage"
    (:`then`
      (`PrimitiveComponent.SetCollisionResponseToChannel` (`self.CapsuleComponent`) "ECC_Pawn" "ECR_Overlap")
      (`PrimitiveComponent.SetCollisionEnabled` (`self.Mesh`) "NoCollision")
      (bind _asgm_fps (cast `/Game/FPSSurvival/ASSETS/Core/GM_FPS` (`GameplayStatics.GetGameMode`)))
      (`/Game/FPSSurvival/ASSETS/Core/GM_FPS.ZombieKilled` _asgm_fps)
      (`KismetSystemLibrary.Delay` 7.0)
      (`self.K2_DestroyActor`))))

(fn `UserConstructionScript`)